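; BP_CoinGameMode is the multiplayer game mode for the coin game, handling player join, leave, player data and session end.
; On login it tracks the controller, spawns a BP_CoinPawn at the first PlayerStart found, possesses and initializes it.
; UpdatePlayerData gathers every player's info, sends the list to each controller and reinitializes their pawns.
; EndSession calls EndClientSession on all PlayerArray controllers, then again on player 0 after a short delay.
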(event Custom|EndSession
  ;[1 1 1] EndSession
  (for _array_element (Variables|/Script/Engine.GameStateBase|GetPlayerArray (Game|GetGameState))
    (if (!= _array_element self)
      (bind _asbp_coin_player_controller (Utilities|Casting|CastToBP_CoinPlayerController (Game|GetPlayerController _array_element)))
      (Default|EndClientSession _asbp_coin_player_controller)))
  (Utilities|FlowControl|Delay 0.2)
  (bind _asbp_coin_player_controller_2 (Utilities|Casting|CastToBP_CoinPlayerController (Game|GetPlayerController 0)))
  (Default|EndClientSession _asbp_coin_player_controller_2))

(event Custom|UpdateCharacter
  (params (SlotIndex :type Integer))
  ;[1 1 1] Update ui and character
  (bind _asbp_coin_pawn (Utilities|Casting|CastToBP_CoinPawn (Pawn|GetControlledPawn (Utilities|Array|Get(acopy) (Variables|Default|GetPlayers) SlotIndex))))
  (Default|InitPawn _asbp_coin_pawn (Utilities|Array|Get(acopy) (Variables|Default|GetPlayersInfo) SlotIndex)))

(event Custom|UpdatePlayerData
  ;[1 1 1] Update ui and character
  (Utilities|Array|Clear (Variables|Default|GetPlayersInfo))
  (for (_array_element _array_index) (Variables|Default|GetPlayers)
    (Utilities|Array|SetArrayElem (Variables|Default|GetPlayersInfo) _array_index (Variables|/Game/Framework/BP_CoinPlayerController.BP_CoinPlayerController_C|GetPlayerInfo _array_element) true))
  (for (_array_element_2 _array_index_2) (Variables|Default|GetPlayers)
    (Default|UpdatePlayersInfo _array_element_2 (Variables|Default|GetPlayersInfo))
    (CallFunction|UpdateCharacter _array_index_2)))

(event EventOnLogout
  (params (ExitingController :type Controller%20Object%20Reference))
  (bind _asbp_coin_player_controller (Utilities|Casting|CastToBP_CoinPlayerController ExitingController))
  (Utilities|Array|RemoveItem (Variables|Default|GetPlayers) _asbp_coin_player_controller))

(event EventBeginPlay
  (bind _asbp_coin_game_state (Utilities|Casting|CastToBP_CoinGameState (Game|GetGameState)))
  (Variables|Default|SetAs%20BP%20Coin%20Game%20State _asbp_coin_game_state))

(event EventPostLogin
  (params (NewPlayer :type Player%20Controller%20Object%20Reference))
  ;[1 1 1] OnPostLogin
  (bind _asbp_coin_player_controller (Utilities|Casting|CastToBP_CoinPlayerController NewPlayer))
  (Utilities|Array|Add (Variables|Default|GetPlayers) _asbp_coin_player_controller)
  (bind _pawn (CallFunction|SpawnPawn _asbp_coin_player_controller))
  (Pawn|Possess _asbp_coin_player_controller _pawn)
  (Default|Init _asbp_coin_player_controller))

(fn ConstructionScript)

(fn SpawnPawn
  (params (PlayerController :type BP%20Coin%20Player%20Controller%20Object%20Reference))
  (bind _returnvalue (Actor|GetActorOfClass "/Script/Engine.PlayerStart"))
  (bind _returnvalue_2 (Game|SpawnActorfromClass "/Game/Framework/BP_CoinPawn.BP_CoinPawn_C" (Transformation|GetActorTransform _returnvalue) "Undefined" "MultiplyWithRoot" PlayerController 0))
  (return _returnvalue_2))