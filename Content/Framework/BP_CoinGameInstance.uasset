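; Game instance for a multiplayer coin game that owns player save data, menu widget creation and LAN sessions.
; Init picks a randomly numbered save slot, then loads or creates its save; name and hat setters save immediately, and hat changes fire a dispatcher.
; Events open custom, server-list and lobby menus, host a listen-server Lobby, join sessions and server-travel between maps.
; Network and travel error handlers are empty.
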(event Custom|CreateSession
  ;[1 1 1] Session Create & Join
  (|Session (Game|GetPlayerController 0) 4 true
    (:OnSuccess
      (Game|OpenLevel(byName) "Lobby" true "listen"))
    (:OnFailure
      (Development|PrintString "Fail to create session"))))

(event Custom|TravelToMap
  (params (MapName :type String))
  (Development|ExecuteConsoleCommand (Utilities|String|Append "servertravel " MapName) (Game|GetPlayerController 0)))

(event Custom|JoinSession
  (params (sessionResult :type Blueprint%20Session%20Result%20Structure))
  ;[1 1 1] Session Create & Join
  (|JoinSession (Game|GetPlayerController 0) sessionResult
    (:OnFailure
      (Development|PrintString "Fail to join session"))))

(event Custom|ShowCustomMenu
  ;[1 1 1] Show UI
  (bind _returnvalue (UserInterface|CreateWidget "/Game/UI/WB_Menu_Custom.WB_Menu_Custom_C"))
  (UserInterface|Viewport|AddtoViewport _returnvalue 0))

(event Custom|ShowServerListMenu
  ;[1 1 1] Show UI
  (bind _returnvalue (UserInterface|CreateWidget "/Game/UI/WB_Menu_ServerList.WB_Menu_ServerList_C"))
  (bind _output_get (Variables|Default|SetServerListUI _returnvalue))
  (UserInterface|Viewport|AddtoViewport _output_get 0))

(event Custom|ShowLobbyMenu
  ;[1 1 1] Show UI
  (bind _returnvalue (UserInterface|CreateWidget "/Game/UI/WB_Menu_Lobby.WB_Menu_Lobby_C"))
  (UserInterface|Viewport|AddtoViewport _returnvalue 0))

(event EventInit
  (Variables|Default|SetSaveSlotName (Utilities|String|Append "PlayerInfo" (Utilities|String|ToString(Integer) (Math|Random|RandomInteger 100))))
  (CallFunction|CheckSaveData))

(event EventHandleNetworkError
  (params (FailureType :type ENetworkFailure%20Enum :default "NetDriverAlreadyExists") (bIsServer :type Boolean)))

(event EventHandleTravelError
  (params (FailureType :type ETravelFailure%20Enum :default "NoLevel")))

(fn LoadPlayerData
  (bind _returnvalue (SaveGame|LoadGamefromSlot (Variables|Default|GetSaveSlotName)))
  (bind _asbp_player_save_data (Utilities|Casting|CastToBP_PlayerSaveData _returnvalue))
  (bind _output_get (Variables|Default|SetPlayerSaveData _asbp_player_save_data))
  (Variables|Default|SetPlayerInfo (Variables|/Game/Data/BP_PlayerSaveData.BP_PlayerSaveData_C|GetPlayerInfo _output_get))
  (return))

(fn SavePlayerData
  (Utilities|IsValid (Variables|Default|GetPlayerSaveData)
    (:Is%20Valid
      _)
    (:Is%20Not%20Valid
      (bind _returnvalue (SaveGame|CreateSaveGameObject "/Game/Data/BP_PlayerSaveData.BP_PlayerSaveData_C"))
      (Variables|Default|SetPlayerSaveData _returnvalue)))
  (Variables|/Game/Data/BP_PlayerSaveData.BP_PlayerSaveData_C|SetPlayerInfo (Variables|Default|GetPlayerSaveData) (Variables|Default|GetPlayerInfo))
  (SaveGame|SaveGametoSlot (Variables|Default|GetPlayerSaveData) (Variables|Default|GetSaveSlotName))
  (return))

(fn SetPlayerHat
  (params (Player%20Info%20Player%20Hat :type E_Hats%20Enum :default "NewEnumerator0"))
  (Variables|Default|SetPlayerInfo (Utilities|Struct|MakeS_PlayerInfo (.playername (Variables|Default|GetPlayerInfo)) Player%20Info%20Player%20Hat))
  (CallFunction|SavePlayerData)
  (Default|CallOnChangePlayerHat Player%20Info%20Player%20Hat))

(fn GetPlayerInfo
  (return (Variables|Default|GetPlayerInfo)))

(fn CheckSaveData
  (bind _returnvalue (SaveGame|DoesSaveGameExist (Variables|Default|GetSaveSlotName)))
  (if _returnvalue
    (CallFunction|LoadPlayerData)
    (else
      (CallFunction|SavePlayerData))))

(fn SetPlayerName
  (params (Player%20Info%20Player%20Name :type Text))
  (Variables|Default|SetPlayerInfo (Utilities|Struct|MakeS_PlayerInfo Player%20Info%20Player%20Name (.playerhat (Variables|Default|GetPlayerInfo))))
  (CallFunction|SavePlayerData))