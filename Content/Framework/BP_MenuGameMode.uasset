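; Game mode for the menu and lobby levels, telling each joining player's controller to show the UI for the current level.
; In the lobby it tracks controllers, shares everyone's player info and spawns or updates a menu pawn for each on a free slot actor.
; Logout destroys the pawn, frees its slot and refreshes the lobby.
; Ending the session notifies all players' controllers, then player zero's again after a short delay.
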(event Custom|EndSession
  ;[1 1 1] EndSession
  (for _array_element (Variables|/Script/Engine.GameStateBase|GetPlayerArray (Game|GetGameState))
    (if (!= _array_element self)
      (bind _asbp_menu_player_controller (Utilities|Casting|CastToBP_MenuPlayerController (Game|GetPlayerController _array_element)))
      (Default|EndClientSession _asbp_menu_player_controller)))
  (Utilities|FlowControl|Delay 0.2)
  (bind _asbp_menu_player_controller_2 (Utilities|Casting|CastToBP_MenuPlayerController (Game|GetPlayerController 0)))
  (Default|EndClientSession _asbp_menu_player_controller_2))

(event Custom|UpdateCharacter
  (params (SlotIndex :type Integer))
  (bind _players (Variables|Default|GetPlayers))
  (bind _output (Utilities|Array|Get(acopy) _players SlotIndex))
  ;[1 1 1] Update ui and character
  (Utilities|IsValid (Variables|/Game/Framework/BP_MenuPlayerController.BP_MenuPlayerController_C|GetPlayerCharacter (Utilities|Array|Get(acopy) (Variables|Default|GetPlayers) SlotIndex))
    (:Is%20Valid
      (Default|UpdatePawn (Variables|/Game/Framework/BP_MenuPlayerController.BP_MenuPlayerController_C|GetPlayerCharacter (Utilities|Array|Get(acopy) (Variables|Default|GetPlayers) SlotIndex)) (Utilities|Array|Get(acopy) (Variables|Default|GetPlayersInfo) SlotIndex)))
    (:Is%20Not%20Valid
      (bind _emptyslot (CallFunction|GetPlayerSlot))
      (Variables|/Game/Blueprints/BP_LobbyPlayerSlot.BP_LobbyPlayerSlot_C|SetIsUsed _emptyslot true)
      (bind _output_get (Variables|/Game/Framework/BP_MenuPlayerController.BP_MenuPlayerController_C|SetPlayerSlot _output _emptyslot))
      (bind _returnvalue (Game|SpawnActorfromClass "/Game/Blueprints/BP_MenuPawn.BP_MenuPawn_C" (Transformation|GetActorTransform _output_get) "Undefined" "MultiplyWithRoot" 0 0))
      (bind _output_get_2 (Variables|/Game/Framework/BP_MenuPlayerController.BP_MenuPlayerController_C|SetPlayerCharacter _output _returnvalue))
      (Utilities|IsValid _output_get_2
        (:Is%20Valid
          (Default|UpdatePawn _output_get_2 (Utilities|Array|Get(acopy) (Variables|Default|GetPlayersInfo) SlotIndex)))))))

(event Custom|UpdateLobby
  ;[1 1 1] Update ui and character
  (Utilities|Array|Clear (Variables|Default|GetPlayersInfo))
  (for (_array_element _array_index) (Variables|Default|GetPlayers)
    (Utilities|Array|SetArrayElem (Variables|Default|GetPlayersInfo) _array_index (Variables|/Game/Framework/BP_MenuPlayerController.BP_MenuPlayerController_C|GetPlayerInfo _array_element) true))
  (for (_array_element_2 _array_index_2) (Variables|Default|GetPlayers)
    (Default|UpdatePlayersInfo _array_element_2 (Variables|Default|GetPlayersInfo))
    (CallFunction|UpdateCharacter _array_index_2)))

(event EventOnLogout
  (params (ExitingController :type Controller%20Object%20Reference))
  ;[1 1 1] On Logout
  (bind _asbp_menu_player_controller (Utilities|Casting|CastToBP_MenuPlayerController ExitingController))
  (Utilities|IsValid (Variables|/Game/Framework/BP_MenuPlayerController.BP_MenuPlayerController_C|GetPlayerCharacter _asbp_menu_player_controller)
    (:Is%20Valid
      (Actor|DestroyActor (Variables|/Game/Framework/BP_MenuPlayerController.BP_MenuPlayerController_C|GetPlayerCharacter _asbp_menu_player_controller))
      (Variables|/Game/Blueprints/BP_LobbyPlayerSlot.BP_LobbyPlayerSlot_C|SetIsUsed (Variables|/Game/Framework/BP_MenuPlayerController.BP_MenuPlayerController_C|GetPlayerSlot _asbp_menu_player_controller) false))
    (:Is%20Not%20Valid
      _))
  (Utilities|Array|RemoveItem (Variables|Default|GetPlayers) _asbp_menu_player_controller)
  (CallFunction|UpdateLobby))

(event EventPostLogin
  (params (NewPlayer :type Player%20Controller%20Object%20Reference))
  ;[1 1 1] OnPostLogin : show ui and init
  (bind _returnvalue (Game|GetCurrentLevelName true))
  (switch string _returnvalue
    (:Default
      (bind _asbp_menu_player_controller (Utilities|Casting|CastToBP_MenuPlayerController NewPlayer :!label _label))
      (Default|ShowCustom _asbp_menu_player_controller))
    (:Menu
      (goto _label))
    (:Lobby
      (bind _asbp_menu_player_controller_2 (Utilities|Casting|CastToBP_MenuPlayerController NewPlayer))
      (Utilities|Array|Add (Variables|Default|GetPlayers) _asbp_menu_player_controller_2)
      (Default|ShowLobby _asbp_menu_player_controller_2)
      (Default|Init _asbp_menu_player_controller_2))))

(fn ConstructionScript)

(fn GetPlayerSlot
  (if (== (Utilities|Array|Length (Variables|Default|GetPlayer%20Slots)) 0)
    (bind _outactors (Actor|GetAllActorsOfClass "/Game/Blueprints/BP_LobbyPlayerSlot.BP_LobbyPlayerSlot_C"))
    (Variables|Default|SetPlayer%20Slots _outactors))
  (for _array_element (Variables|Default|GetPlayer%20Slots)
    (if (not (Variables|/Game/Blueprints/BP_LobbyPlayerSlot.BP_LobbyPlayerSlot_C|GetIsUsed _array_element))
      (return _array_element)))
  (return 0))