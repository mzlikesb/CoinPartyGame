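; Player controller for a multiplayer coin game that manages the local game HUD, pause menu and player info.
; Init loads saved player info from the game instance's save slot, sends it through a server update event to the game mode, and sets the HUD name.
; Update events refresh HUD player names and coin display.
; Pause input flip-flops between lazily created widgets, switching input mode, and ending the client session returns to Menu.
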(event Custom|UpdatePlayersInfo
  (params (PlayersInfo :type Array%20of%20S%20Player%20Info%20Structures))
  ;[1 1 1] InitData
  (CallFunction|CreateGameUI)
  (Default|UpdatePlayerNames (Variables|Default|GetGameUI) PlayersInfo))

(event Custom|EndClientSession
  ;[1 1 1] EndSession
  (|DestroySession self
    (:then
      (Game|OpenLevel(byName) "Menu"))))

(event Custom|Init
  ;[1 1 1] InitData
  (bind _playerinfo (CallFunction|LoadPlayerData))
  (CallFunction|UpdatePlayerDataServer _playerinfo)
  (CallFunction|CreateGameUI)
  (Default|SetPlayerName (Variables|Default|GetGameUI) (.PlayerName (Utilities|Struct|BreakS_PlayerInfo _playerinfo))))

(event Custom|UpdateCoin
  (params (Coin :type Integer))
  (Default|UpdateCoin (Variables|Default|GetGameUI) Coin))

(event Custom|UpdatePlayerData_Server
  (params (PlayerInfo :type S%20Player%20Info%20Structure))
  ;[1 1 1] InitData
  (Variables|Default|SetPlayerInfo PlayerInfo)
  (bind _asbp_coin_game_mode (Utilities|Casting|CastToBP_CoinGameMode (Game|GetGameMode)))
  (Default|UpdatePlayerData _asbp_coin_game_mode))

(event Input|EnhancedActionEvents|EnhancedInputActionIA_Pause
  (params (ActionValue :type Boolean) (ElapsedSeconds :type Float%20%28double-precision%29) (TriggeredSeconds :type Float%20%28double-precision%29) (InputAction :type Input%20Action%20Object%20Reference :default "/Game/Input/Actions/IA_Pause.IA_Pause"))
  (Utilities|FlowControl|FlipFlop
    (:A
      (CallFunction|ShowPauseUI))
    (:B
      (CallFunction|ShowGameUI))))

(event EventBeginPlay
  (CallFunction|ShowGameUI))

(fn ConstructionScript)

(fn LoadPlayerData
  (bind _asbp_coin_game_instance (Utilities|Casting|CastToBP_CoinGameInstance (Game|GetGameInstance)))
  (bind _returnvalue (SaveGame|LoadGamefromSlot (Variables|/Game/Framework/BP_CoinGameInstance.BP_CoinGameInstance_C|GetSaveSlotName _asbp_coin_game_instance)))
  (bind _asbp_player_save_data (Utilities|Casting|CastToBP_PlayerSaveData _returnvalue))
  (return (Variables|/Game/Data/BP_PlayerSaveData.BP_PlayerSaveData_C|GetPlayerInfo _asbp_player_save_data)))

(fn ShowGameUI
  (bind _self self)
  (if (Pawn|IsLocalController)
    (Viewport|RemoveAllWidgets)
    (CallFunction|CreateGameUI)
    (UserInterface|Viewport|AddtoViewport (Variables|Default|GetGameUI) 0)
    (Input|SetInputModeGameOnly _self false)
    (Variables|Default|SetbShowMouseCursor _self false)
    (return)))

(fn ShowPauseUI
  (Viewport|RemoveAllWidgets)
  (Utilities|IsValid (Variables|Default|GetPauseUI)
    (:Is%20Valid
      _)
    (:Is%20Not%20Valid
      (bind _returnvalue (UserInterface|CreateWidget "/Game/UI/WB_Pause.WB_Pause_C" 0 (Networking|IsServer)))
      (bind _output_get (Variables|Default|SetPauseUI _returnvalue))))
  (UserInterface|Viewport|AddtoViewport _output_get 0)
  (Input|SetInputModeGameandUI self 0 "DoNotLock" true false)
  (Variables|Default|SetbShowMouseCursor true)
  (return))

(fn CreateGameUI
  (Utilities|IsValid (Variables|Default|GetGameUI)
    (:Is%20Valid
      _)
    (:Is%20Not%20Valid
      (bind _returnvalue (UserInterface|CreateWidget "/Game/UI/WB_Game.WB_Game_C" self))
      (Variables|Default|SetGameUI _returnvalue)))
  (return))