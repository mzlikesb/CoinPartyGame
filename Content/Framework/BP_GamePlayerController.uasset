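; Player controller that manages the in-game HUD, chat, player data registration and game-over screen.
; On BeginPlay the local controller adds the mode widget and a lazily created, cached game UI, which receives chat, coin and player-name updates.
; SendChat relays formatted messages to every controller.
; Init reads player data from the GameInstance, then notifies GameMode, names the PlayerState and registers with GameState.
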(event Custom|SendChat
  (params (PlayerName :type Text) (ChatMessage :type Text))
  ;[1 1 1] 채팅 기능
  (bind _outactors (Actor|GetAllActorsOfClass "BP_GamePlayerController_C"))
  (for _array_element _outactors
    (CallFunction|RecieveChat _array_element (Utilities|Text|FormatText "{player} : {message}" PlayerName ChatMessage))))

(event Custom|RecieveChat
  (params (ChatMessage :type Text))
  ;[1 1 1] 채팅 기능
  (bind _gameui (CallFunction|GetGameUI))
  (Default|OnRecieveChat _gameui ChatMessage))

(event Custom|UpdateCoin
  (params (NumberOfCoin :type Integer))
  (bind _gameui (CallFunction|GetGameUI))
  (Default|UpdateCoins _gameui NumberOfCoin))

(event Custom|Init
  ;[1 1 1] 플레이어 데이터 로드 및 초기화
  (bind _asbp_game_instance (Utilities|Casting|CastToBP_GameInstance (Game|GetGameInstance)))
  (CallFunction|UpdatePlayerData (Variables|/Game/Framework/BP_GameInstance.BP_GameInstance_C|GetPlayerData _asbp_game_instance)))

(event Custom|UpdatePlayerData
  (params (PlayerData :type S%20Player%20Data%20Structure))
  ;[1 1 1] 플레이어 데이터 로드 및 초기화
  (bind _output_get (Variables|Default|SetPlayerData PlayerData))
  (bind _asbp_game_mode (Utilities|Casting|CastToBP_GameMode (Game|GetGameMode)))
  (Default|UpdatePlayerData _asbp_game_mode)
  (bind _asbp_game_player_state (Utilities|Casting|CastToBP_GamePlayerState (Variables|GetPlayerState)))
  (bind _output_get_2 (Default|SetPlayerName _asbp_game_player_state (.PlayerName (Utilities|Struct|BreakS_PlayerData _output_get))))
  (bind _asbp_game_state (Utilities|Casting|CastToBP_GameState (Game|GetGameState)))
  (Default|AddPlayer _asbp_game_state _output_get_2))

(event Custom|UpdateAllPlayerData
  (params (PlayerData :type Array%20of%20S%20Player%20Data%20Structures))
  (bind _gameui (CallFunction|GetGameUI))
  (Default|UpdatePlayerNames _gameui PlayerData))

(event Custom|ShowGameOver
  (params (ScoreList :type Array%20of%20S%20Player%20Score%20Structures))
  (Viewport|RemoveAllWidgets)
  (bind _returnvalue (UserInterface|CreateWidget "/Game/UI/WB_GameOver.WB_GameOver_C"))
  (UserInterface|Viewport|AddtoViewport _returnvalue 0)
  (Default|SetScore _returnvalue ScoreList))

(event EventBeginPlay
  (if (Pawn|IsLocalController)
    (bind _returnvalue (UserInterface|CreateWidget "/Game/UI/WB_Mode.WB_Mode_C"))
    (bind _output_get (Variables|Default|SetMode _returnvalue))
    (UserInterface|Viewport|AddtoViewport _output_get 0)
    (bind _gameui (CallFunction|GetGameUI))
    (UserInterface|Viewport|AddtoViewport _gameui 0)))

(fn ConstructionScript)

(fn GetGameUI
  (Utilities|IsValid (Variables|Default|GetGameUI)
    (:Is%20Valid
      _)
    (:Is%20Not%20Valid
      (bind _returnvalue (UserInterface|CreateWidget "/Game/UI/WB_GameUI.WB_GameUI_C"))
      (Variables|Default|SetGameUI _returnvalue)))
  (return (Variables|Default|GetGameUI)))