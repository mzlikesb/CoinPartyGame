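; BP_GameState is the game state Blueprint that holds all player scores and runs the match countdown timer.
; GameStart resets the countdown to the time limit, and Tick decrements it while the game is active.
; When time runs out, GameOver sets the game-over flag and forwards the call to BP_GameMode.
; AddPlayer appends score entries, and UpdateScore overwrites them using ClientID as the array index.
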(event Custom|GameStart
  (Variables|Default|SetCurrentTime (Variables|Default|GetLimitTime))
  (Variables|Default|SetIsGameOver false))

(event Custom|GameOver
  (Variables|Default|SetIsGameOver true)
  (bind _asbp_game_mode (Utilities|Casting|CastToBP_GameMode (Game|GetGameMode)))
  (Default|GameOver _asbp_game_mode))

(event Custom|UpdateScore
  (params (PlayerScore :type S%20Player%20Score%20Structure))
  (Utilities|Array|SetArrayElem (Variables|Default|GetAllPlayerScores) (.ClientID (Utilities|Struct|BreakS_PlayerScore PlayerScore)) PlayerScore))

(event Custom|AddPlayer
  (params (NewPlayerScore :type S%20Player%20Score%20Structure%20%28by%20ref%29))
  (Utilities|Array|Add (Variables|Default|GetAllPlayerScores) NewPlayerScore))

(event EventTick
  (params (DeltaSeconds :type Float%20%28single-precision%29))
  (if (not (Variables|Default|GetIsGameOver))
    (Variables|Default|SetCurrentTime (- (Variables|Default|GetCurrentTime) DeltaSeconds))
    (if (<= (Variables|Default|GetCurrentTime) 0.0)
      (CallFunction|GameOver))))

(fn ConstructionScript)