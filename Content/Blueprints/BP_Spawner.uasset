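; Spawner actor that scatters a configurable number of actors of a chosen class inside a box volume when play begins, on the server only.
; Spawn first runs Dispose to destroy and clear earlier spawns, then places each new actor at a random point within the box extents, adjusting for collisions, and tracks it in SpawnedActors.
; A HideAllCoins event destroys every tracked actor without clearing the array, suggesting the spawned items are coins.
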(event Custom|HideAllCoins
  (for _array_element (Variables|Default|GetSpawnedActors)
    (Actor|DestroyActor _array_element)))

(event EventBeginPlay
  (Networking|SwitchHasAuthority
    (:Authority
      (CallFunction|Spawn))))

(event Collision|EventActorBeginOverlap
  (params (OtherActor :type Actor%20Object%20Reference)))

(event EventTick
  (params (DeltaSeconds :type Float%20%28single-precision%29)))

(fn ConstructionScript)

(fn Spawn
  (bind _box (Variables|Default|GetBox))
  (bind _boxextent (Variables|/Script/Engine.BoxComponent|GetBoxExtent _box))
  (CallFunction|Dispose)
  (for _index (range 0 (Variables|Default|GetSpawnNumber))
    (bind _returnvalue (Game|SpawnActorfromClass (Variables|Default|GetSpawnActor) (Math|Transform|MakeTransform (Math|Random|RandomPointinBoundingBox (Transformation|GetWorldLocation _box) (Math|Vector|MakeVector (.x _boxextent) (.y _boxextent) 0.0)) "0, 0, 0" "1.000000,1.000000,1.000000") "AdjustIfPossibleButAlwaysSpawn" "MultiplyWithRoot" 0 0))
    (Utilities|Array|Add (Variables|Default|GetSpawnedActors) _returnvalue)))

(fn Dispose
  (for _array_element (Variables|Default|GetSpawnedActors)
    (Actor|DestroyActor _array_element))
  (Utilities|Array|Clear (Variables|Default|GetSpawnedActors)))