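; BP_MenuPawn is a menu pawn that displays a player's hat and name.
; On BeginPlay it casts the game instance to BP_CoinGameInstance and binds ChangeHat to its hat-change event, which swaps the static mesh between fruit and vegetable hats or none.
; UpdatePawn takes a PlayerInfo, applies the same hat-to-mesh selection and writes the player name to a text render.
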(event Custom|ChangeHat
  (params (Hat :type E_Hats%20Enum :default "NewEnumerator0"))
  (Components|StaticMesh|SetStaticMesh (Variables|Default|GetStaticMesh) (Utilities|Select :Index Hat :NewEnumerator0 0 :NewEnumerator1 "/Game/Assets/Models/apple.apple" :NewEnumerator2 "/Game/Assets/Models/banana.banana" :NewEnumerator3 "/Game/Assets/Models/carrot.carrot")))

(event Custom|UpdatePawn
  (params (PlayerInfo :type S%20Player%20Info%20Structure))
  (bind (_playername _playerhat) (Utilities|Struct|BreakS_PlayerInfo PlayerInfo))
  (Components|StaticMesh|SetStaticMesh (Variables|Default|GetStaticMesh) (Utilities|Select :Index _playerhat :NewEnumerator0 0 :NewEnumerator1 "/Game/Assets/Models/apple.apple" :NewEnumerator2 "/Game/Assets/Models/banana.banana" :NewEnumerator3 "/Game/Assets/Models/carrot.carrot"))
  (Rendering|Components|TextRender|SetText (Variables|Default|GetTextRender) _playername))

(event EventBeginPlay
  (bind _asbp_coin_game_instance (Utilities|Casting|CastToBP_CoinGameInstance (Game|GetGameInstance)))
  (Variables|Default|SetAs%20BP%20Coin%20Game%20Instance _asbp_coin_game_instance)
  (EventDispatchers|BindEventtoOnChangePlayerHat (Variables|Default|GetAs%20BP%20Coin%20Game%20Instance) (delegate Custom|ChangeHat)))

(fn ConstructionScript)