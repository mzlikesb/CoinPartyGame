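; BP_Floor is a moving floor that travels along its Arrow component's forward direction.
; On BeginPlay, only the authority stores the initial location and starts MoveLoop.
; A Timeline's Movement track, scaled by a constant, offsets the actor from that location without sweeping, and restarts from the beginning whenever it finishes, looping endlessly.
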(event Custom|MoveLoop
  ;[1 1 1] 위치 애니메이션 루프
  (bind _movement (Timeline|Timeline PlayFromStart)
    (:Update
      (Transformation|SetActorLocation (+ (Variables|Default|GetInitialPosition) (* (* _movement 1e+02) (Math|Vector|GetForwardVector (Variables|Default|GetArrow)))) false false))
    (:Finished
      (CallFunction|MoveLoop))))

(event EventBeginPlay
  ;[1 1 1] 서버에서만 floor 이동
  (Networking|SwitchHasAuthority
    (:Authority
      (Variables|Default|SetInitialPosition (Transformation|GetActorLocation))
      (CallFunction|MoveLoop))))

(fn ConstructionScript)